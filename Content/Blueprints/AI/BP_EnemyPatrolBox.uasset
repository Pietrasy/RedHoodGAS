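; BP_EnemyPatrolBox is a trigger actor that gives a group of patrolling enemies the player as their combat target while the player is inside it.
; Begin and end overlap events check whether the overlapping actor implements BPI_Player.
; For a player, it loops over the valid entries in PatrolEnemies and sends SetCombatTargetMessage, passing the player on entry and nothing on exit to clear the target.
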(event `self.ReceiveActorBeginOverlap`
  (params (OtherActor :type "Actor Object Reference"))
  (`self.PassPlayerAsCombatTarget` OtherActor))

(event `self.ReceiveActorEndOverlap`
  (params (OtherActor :type "Actor Object Reference"))
  (`self.ClearPlayerAsCombatTarget` OtherActor))

(fn `ClearPlayerAsCombatTarget`
  (params (Actor :type "Actor Object Reference"))
  (locals (OverlappedActor :type "Actor Object Reference"))
  (`self.CheckIfActorIsPlayer` Actor
    (:`True`
      (for _array_element (`self.PatrolEnemies`)
        (`/Engine/EditorBlueprintResources/StandardMacros.IsValid` _array_element
          (:`Is Valid`
            (message `/Game/Blueprints/Interfaces/BPI_Enemy.SetCombatTarget` _array_element null))))
      (return))))

(fn `PassPlayerAsCombatTarget`
  (params (Actor :type "Actor Object Reference"))
  (locals (OverlappedActor :type "Actor Object Reference"))
  (`self.CheckIfActorIsPlayer` Actor
    (:`True`
      (for _array_element (`self.PatrolEnemies`)
        (`/Engine/EditorBlueprintResources/StandardMacros.IsValid` _array_element
          (:`Is Valid`
            (message `/Game/Blueprints/Interfaces/BPI_Enemy.SetCombatTarget` _array_element (`local.OverlappedActor`)))))
      (return))))

(fn `UserConstructionScript`)
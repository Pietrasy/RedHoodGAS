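; BP_BaseCharacter is a base character Blueprint providing melee attack detection and hit reactions for PaperZD-animated 2D characters.
; CallAttackBoxTrace runs an object-type box trace between two scene points and sends the hit actor a hit-react message, without checking whether anything was hit.
; Attack and hit-react functions play their sequences as PaperZD animation overrides.
; GetHit only triggers the hit-react animation, with no damage logic.
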(event `/Game/Blueprints/Interfaces/BPI_Character.CallAttackBoxTrace`
  (bind _outhit (`self.AttackBoxTrace`))
  (message `/Game/Blueprints/Interfaces/BPI_Character.CallPlayHitReactAnimation` (`.HitActor` (`GameplayStatics.BreakHitResult` _outhit))))

(fn `AttackBoxTrace`
  (returns (OutHit :type "HitResult Structure") (ReturnValue :type Boolean))
  (bind (_outhit _returnvalue) (`KismetSystemLibrary.BoxTraceSingleForObjects` (`SceneComponent.K2_GetComponentLocation` (`self.BoxTraceStart`)) (`SceneComponent.K2_GetComponentLocation` (`self.BoxTraceEnd`)) (`self.TarceExtent`) (`self.BoxRotation`) (`self.TraceObjectTypes`)))
  (return _outhit _returnvalue))

(fn `GetHit`
  (`self.PlayHitReactAnimation`))

(fn `PlayAttackAnimation`
  (`PaperZDAnimInstance.K2_PlayAnimationOverride` (`PaperZDAnimationComponent.AnimInstance` (`self.PaperZDAnimation`)) (`self.AttackAnimSequence`) "DefaultSlot" 1.0 0.0)
  (return))

(fn `PlayHitReactAnimation`
  (`PaperZDAnimInstance.K2_PlayAnimationOverride` (`PaperZDAnimationComponent.AnimInstance` (`self.PaperZDAnimation`)) (`self.HitReactAnimSequence`) "DefaultSlot" 1.0 0.0)
  (return))

(fn `UserConstructionScript`)
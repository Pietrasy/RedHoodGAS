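; BP_RedHood is the Red Hood character Blueprint, with side-scroller style facing along the X axis.
; RotateCharacter reads the X sign of movement acceleration and snaps control rotation yaw forward or backward, keeping the current facing at zero.
; A CallPlayHitReactAnimation event triggers the hit react animation, and the construction script only runs the parent's.
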(event `/Game/Blueprints/Interfaces/BPI_Character.CallPlayHitReactAnimation`
  (`self.PlayHitReactnimation`))

(fn `RotateCharacter`
  (bind _returnvalue_x (`KismetMathLibrary.BreakVector` (`CharacterMovementComponent.GetCurrentAcceleration` (`self.CharacterMovement`))))
  (`/Engine/EditorBlueprintResources/StandardMacros.CompareFloat` _returnvalue_x
    (:`>`
      (`Controller.SetControlRotation` (`self.GetController`) (`KismetMathLibrary.MakeRotator` 0.0)))
    (:`<`
      (`Controller.SetControlRotation` (`self.GetController`) (`KismetMathLibrary.MakeRotator` 0.0 0.0 180.0)))))

(fn `UserConstructionScript`
  (`parent.UserConstructionScript`))
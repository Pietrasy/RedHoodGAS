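; Player controller for the Red Hood character that handles single-axis movement, jumping and melee combo input.
; It adds the Enhanced Input mapping context, caches the character, and blocks moving and jumping while attacking.
; The first attack requires being grounded; presses during an externally set attack window queue the next combo hit.
; HandleAttackReset then advances through the character's AttackAnimData or resets the combo when none is queued.
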(event `self.ReceiveBeginPlay`
  (`self.SetContextMapping`)
  (`self.CachePlayerCharacter`))

(event `EnhancedInput|/Game/Inputs/Actions/IA_Move`
  (params (ActionValue :type "Float (double-precision)") (ElapsedSeconds :type "Float (double-precision)") (TriggeredSeconds :type "Float (double-precision)") (InputAction :type "InputAction Object Reference" :default "/Game/Inputs/Actions/IA_Move.IA_Move"))
  (:`Triggered`
    (if (not (`/Game/Blueprints/Characters/RedHood/BP_RedHood.IsAttacking` (`self.PlayerCharacter`)))
      (`/Game/Blueprints/Characters/RedHood/BP_RedHood.RotateCharacter` (`self.PlayerCharacter`))
      (`Pawn.AddMovementInput` (`self.PlayerCharacter`) (1.0 0.0 0.0) ActionValue false))))

(event `EnhancedInput|/Game/Inputs/Actions/IA_Jump`
  (params (ActionValue :type Boolean) (ElapsedSeconds :type "Float (double-precision)") (TriggeredSeconds :type "Float (double-precision)") (InputAction :type "InputAction Object Reference" :default "/Game/Inputs/Actions/IA_Jump.IA_Jump"))
  (:`Started`
    (if (not (`/Game/Blueprints/Characters/RedHood/BP_RedHood.IsAttacking` (`self.PlayerCharacter`)))
      (`Character.Jump` (`self.PlayerCharacter`)))))

(event `EnhancedInput|/Game/Inputs/Actions/IA_Attack`
  (params (ActionValue :type Boolean) (ElapsedSeconds :type "Float (double-precision)") (TriggeredSeconds :type "Float (double-precision)") (InputAction :type "InputAction Object Reference" :default "/Game/Inputs/Actions/IA_Attack.IA_Attack"))
  (:`Started`
    (if (`self.IsAttackWindowOpen`)
      (set `self.IsComboActivated` true)
      (elif (not (`NavMovementComponent.IsFalling` (`Character.CharacterMovement` (`self.PlayerCharacter`))))
        (`self.PlayFirstAttack`)))))

(fn `CachePlayerCharacter`
  (bind _asbp_red_hood (cast `/Game/Blueprints/Characters/RedHood/BP_RedHood` (`GameplayStatics.GetPlayerCharacter` 0)))
  (set `self.PlayerCharacter` _asbp_red_hood)
  (return))

(fn `HandleAttackReset`
  (if (`self.IsComboActivated`)
    (`self.StartCombo`)
    (else
      (set `/Game/Blueprints/Characters/RedHood/BP_RedHood.IsAttacking` false (`self.PlayerCharacter`))
      (set `self.AttackCount` 0))))

(fn `IncrementAttackCount`
  (returns (ShouldResetAttackCount :type Boolean))
  (bind _result (`/Engine/EditorBlueprintResources/StandardMacros.IncrementInt` (`self.AttackCount`))
    (:`  `
      (return (> _result (- (`KismetArrayLibrary.Array_Length` (`/Game/Blueprints/Characters/RedHood/BP_RedHood.AttackAnimData` (`self.PlayerCharacter`))) 1))))))

(fn `PlayFirstAttack`
  (if (not (`/Game/Blueprints/Characters/RedHood/BP_RedHood.IsAttacking` (`self.PlayerCharacter`)))
    (set `/Game/Blueprints/Characters/RedHood/BP_RedHood.IsAttacking` true (`self.PlayerCharacter`))
    (`/Game/Blueprints/Characters/RedHood/BP_RedHood.PlayComboAttack` (`self.PlayerCharacter`) 0)
    (return)))

(fn `SetAttackWindow`
  (params (IsAttackWindowOpen :type Boolean))
  (set `self.IsAttackWindowOpen` IsAttackWindowOpen)
  (return))

(fn `SetContextMapping`
  (`EnhancedInputSubsystemInterface.AddMappingContext` (subsystem `EnhancedInputLocalPlayerSubsystem`) "/Game/Inputs/IMC_RedHood.IMC_RedHood" 0 (struct))
  (return))

(fn `SetVariablesToDefault`
  (set `self.IsComboActivated` false)
  (set `self.AttackCount` 0)
  (set `self.IsAttackWindowOpen` false)
  (return))

(fn `StartCombo`
  (bind _shouldresetattackcount (`self.IncrementAttackCount`))
  (if _shouldresetattackcount
    (set `/Game/Blueprints/Characters/RedHood/BP_RedHood.IsAttacking` false (`self.PlayerCharacter`))
    (set `self.AttackCount` 0)
    (set `self.IsComboActivated` false)
    (return)
    (else
      (`/Game/Blueprints/Characters/RedHood/BP_RedHood.PlayComboAttack` (`self.PlayerCharacter`) (`self.AttackCount`))
      (set `self.IsComboActivated` false)
      (return))))

(fn `UserConstructionScript`)